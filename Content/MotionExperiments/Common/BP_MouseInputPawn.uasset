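; BP_MouseInputPawn is a pawn that moves and looks around only while the right mouse button is held, showing the cursor otherwise.
; SetMovementEnabled toggles the movement component's tick, controller-driven rotation and cursor visibility together.
; On enable, it copies the root's world rotation to the control rotation so the view resumes from the current orientation.
; BeginPlay starts with movement disabled and prints an on-screen control hint.
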(event `self.ReceiveBeginPlay`
  (`self.SetMovementEnabled` false)
  (`KismetSystemLibrary.PrintString` "Hold RIGHT CLICK to look around or move" true true (struct :`R` 1.0 :`G` 0.180739 :`A` 1.0) 7.0))

(event `Key|RightMouseButton`
  (params (Key :type "Key Structure"))
  ;[1 1 1] Toggle Movement
  (:`Pressed`
    (`self.SetMovementEnabled` true))
  (:`Released`
    (`self.SetMovementEnabled` false)))

(event `SetMovementEnabled`
  (params (MovementEnabled :type Boolean))
  ;[1 1 1] Toggle Movement
  (bind _output_get (set `self.IsMovementEnabled` MovementEnabled))
  (`ActorComponent.SetComponentTickEnabled` (`self.MovementComponent`) _output_get)
  (bind _output_get_2 (set `self.bUseControllerRotationRoll` (`self.IsMovementEnabled`))) ; Those can also be set in camera
  (bind _output_get_3 (set `self.bUseControllerRotationYaw` _output_get_2))
  (set `self.bUseControllerRotationPitch` _output_get_3)
  ;;[1 1 1] Show/Hide mouse cursor
  (bind _asplayer_controller (cast `PlayerController` (`self.GetController`)))
  (set `PlayerController.bShowMouseCursor` (not (`self.IsMovementEnabled`)) _asplayer_controller)
  ;;[1 1 1] Resume rotation
  (if (`self.IsMovementEnabled`)
    (`Controller.SetControlRotation` (`self.GetController`) (`SceneComponent.K2_GetComponentRotation` (`self.RootComponent`)))))

(fn `UserConstructionScript`)