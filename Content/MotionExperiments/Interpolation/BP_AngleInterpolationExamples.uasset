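; Demo actor comparing angle interpolation methods by rolling three cubes toward a shared TargetAngle.
; Tick drives one cube with critically damped AngleSpringInterpCD, one with AngleInterpTo (both custom C++), and one without interpolation.
; A looping timer randomizes the target beyond a full turn to exercise angle wrapping, when RandomEnabled is set.
; SetTargetAtMousePosition instead derives the target from a mouse-ray and vertical-plane intersection, with debug drawing.
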(event `self.ReceiveBeginPlay`
  ;[1 1 1] Init
  (`self.InitRandomPosition`)
  (for _array_element (`self.K2_GetComponentsByClass` "/Script/Engine.ArrowComponent")
    (`PrimitiveComponent.SetCastShadow` _array_element false)))

(event `self.ReceiveTick`
  (params (DeltaSeconds :type "Float (single-precision)"))
  (bind _cube11 (`self.Cube11`))
  (bind _cube (`self.Cube`))
  (bind _relativerotation_roll (`KismetMathLibrary.BreakRotator` (`SceneComponent.RelativeRotation` _cube)))
  (bind _relativerotation_roll_2 (`KismetMathLibrary.BreakRotator` (`SceneComponent.RelativeRotation` _cube11)))
  (`|ExecutionSequence`
    (:`then_0`
      ;[0 0.01771 0.004418] Critically Damped Spring (AngleSpringInterpCD: Custom from InterploationLibrary.cpp)
      (`SceneComponent.K2_SetRelativeRotation` _cube (`KismetMathLibrary.MakeRotator` (`InterpolationLibrary.AngleSpringInterpCD` _relativerotation_roll (`self.TargetAngle`) (`self.SpringVelocity`) DeltaSeconds)) false false))
    (:`then_3`
      ;[1 1 1] AngleInterpTo (Custom from InterploationLibrary.cpp)
      (`SceneComponent.K2_SetRelativeRotation` _cube11 (`KismetMathLibrary.MakeRotator` (`InterpolationLibrary.AngleInterpTo` _relativerotation_roll_2 (`self.TargetAngle`) DeltaSeconds)) false false))
    (:`then_4`
      ;[1 1 1] No Interpolation
      (`SceneComponent.K2_SetRelativeRotation` (`self.Cube111`) (`KismetMathLibrary.MakeRotator` (`self.TargetAngle`)) false false))))

(event `InitRandomPosition`
  ;[1 1 1] Random rotation
  (`KismetSystemLibrary.Delay` 0.5)
  (`KismetSystemLibrary.K2_SetTimerDelegate` (delegate `RandomTarget`) 1.0 true))

(event `RandomTarget`
  ;[1 1 1] Random rotation
  (if (`self.RandomEnabled`)
    (bind _output_get (set `self.TargetAngle` (`KismetMathLibrary.RandomFloatInRange` -720.0 720.0)))
    (`KismetSystemLibrary.PrintString` (`KismetStringLibrary.Conv_DoubleToString` _output_get))))

(event `SetTargetAtMousePosition`
  (bind _returnvalue (`GameplayStatics.GetPlayerController` 0))
  (bind _returnvalue_x (`KismetMathLibrary.BreakVector` (`self.K2_GetActorLocation`)))
  (bind _defaultsceneroot (`self.DefaultSceneRoot`))
  (bind (_locationx _locationy) (`PlayerController.GetMousePosition` _returnvalue))
  (bind _returnvalue_2 (`SceneComponent.K2_GetComponentLocation` _defaultsceneroot))
  (bind (_worldposition _worlddirection) (`GameplayStatics.DeprojectScreenToWorld` _returnvalue (`KismetMathLibrary.MakeVector2D` _locationx _locationy)))
  (bind _returnvalue_3 (+ (`.Intersection` (`KismetMathLibrary.LinePlaneIntersection` _worldposition (+ _worldposition (* _worlddirection 10000.0)) (make `Plane` _returnvalue_x 1.0))) (-150.0 0.0 0.0)))
  (bind (_returnvalue_roll _returnvalue_pitch _returnvalue_yaw) (`KismetMathLibrary.BreakRotator` (`KismetMathLibrary.InverseTransformRotation` (`SceneComponent.K2_GetComponentToWorld` _defaultsceneroot) (`KismetMathLibrary.FindLookAtRotation` _returnvalue_2 _returnvalue_3))))
  ;[1 1 1] Set target from mouse / plane intersection
  ;[1 1 1] World location to relative target in blueprint
  (set `self.TargetAngle` _returnvalue_yaw :!pinned true) ; Not 360 but got other things to do ;)
  (`KismetSystemLibrary.DrawDebugPoint` _returnvalue_3 10.0 (struct :`R` 1.0 :`B` 0.335471 :`A` 1.0))
  (`KismetSystemLibrary.DrawDebugSphere` _returnvalue_2 60.0 3 (struct :`R` 0.291667 :`B` 0.133423 :`A` 1.0) 0.0 5.0))

(fn `UserConstructionScript`)