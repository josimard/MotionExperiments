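; Demo actor that compares float interpolation methods side by side by moving components along local Y toward a shared target.
; Tick drives a custom critically damped spring, FloatSpringInterp with clamped delta time, FInterpTo and an uninterpolated reference, plus a debug line at the target.
; The target is randomized on a looping timer when enabled, or set by intersecting the mouse ray with a vertical plane, avoiding physics raycasts.
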(event `self.ReceiveBeginPlay`
  ;[1 1 1] Init
  (`self.InitRandomPosition`))

(event `self.ReceiveTick`
  (params (DeltaSeconds :type "Float (single-precision)"))
  (bind _nointerpolation (`self.NoInterpolation`))
  (bind _floatspringinterp (`self.FloatSpringInterp`))
  (bind _floatspringinterpcd (`self.FloatSpringInterpCD`))
  (bind _finterpto (`self.FInterpTo`))
  (bind (_relativelocation_x _relativelocation_y _relativelocation_z) (`KismetMathLibrary.BreakVector` (`SceneComponent.RelativeLocation` _nointerpolation)))
  (bind (_relativelocation_x_2 _relativelocation_y_2 _relativelocation_z_2) (`KismetMathLibrary.BreakVector` (`SceneComponent.RelativeLocation` _floatspringinterp)))
  (bind (_relativelocation_x_3 _relativelocation_y_3 _relativelocation_z_3) (`KismetMathLibrary.BreakVector` (`SceneComponent.RelativeLocation` _floatspringinterpcd)))
  (bind (_relativelocation_x_4 _relativelocation_y_4 _relativelocation_z_4) (`KismetMathLibrary.BreakVector` (`SceneComponent.RelativeLocation` _finterpto)))
  (bind _returnvalue (`KismetMathLibrary.TransformLocation` (`self.GetTransform`) (`KismetMathLibrary.MakeVector` 0.0 (`self.RelativeTargetY`))))
  (`|ExecutionSequence`
    (:`then_0`
      ;[0 0.01771 0.004418] FloatSpringInterpCD: Critically Damped Spring (Custom from InterploationLibrary.cpp)
      (`SceneComponent.K2_SetRelativeLocation` _floatspringinterpcd (`KismetMathLibrary.MakeVector` 0.0 (`InterpolationLibrary.FloatSpringInterpCD` _relativelocation_y_3 (`self.RelativeTargetY`) (`self.SpringVelocityCD`) DeltaSeconds) _relativelocation_z_3) false false))
    (:`then_2`
      ;[1 1 1] FloatSpringInterp (With Critical damping factor at 1!)
      (bind _returnvalue_2 (`KismetMathLibrary.FloatSpringInterp` _relativelocation_y_2 (`self.RelativeTargetY`) (`self.SpringInterpState`) 10.0 1.0 (`KismetMathLibrary.FMin` DeltaSeconds 0.1)))
      (`SceneComponent.K2_SetRelativeLocation` _floatspringinterp (`KismetMathLibrary.MakeVector` 0.0 _returnvalue_2 _relativelocation_z_2) false false))
    (:`then_3`
      ;[1 1 1] FInterpTo
      (`SceneComponent.K2_SetRelativeLocation` _finterpto (`KismetMathLibrary.MakeVector` 0.0 (`KismetMathLibrary.FInterpTo` _relativelocation_y_4 (`self.RelativeTargetY`) DeltaSeconds 5.0) _relativelocation_z_4) false false))
    (:`then_4`
      ;[1 1 1] No Interpolation
      (`SceneComponent.K2_SetRelativeLocation` _nointerpolation (`KismetMathLibrary.MakeVector` 0.0 (`self.RelativeTargetY`) _relativelocation_z) false false))
    (:`then_5`
      ;[1 1 1] Debug Line
      (`KismetSystemLibrary.DrawDebugLine` (+ _returnvalue (0.0 0.0 -1000.0)) (+ _returnvalue (0.0 0.0 1000.0)) (struct :`R` 1.0 :`G` 1.0 :`B` 1.0 :`A` 1.0) 0.0 5.0))))

(event `InitRandomPosition`
  ;[1 1 1] Random position each X seconds
  (`KismetSystemLibrary.Delay` 1.0)
  (`KismetSystemLibrary.K2_SetTimerDelegate` (delegate `RandomTarget`) 0.7 true))

(event `RandomTarget`
  ;[1 1 1] Random position each X seconds
  (if (`self.RandomEnabled`)
    (set `self.RelativeTargetY` (* (`KismetMathLibrary.RandomFloat`) (.y (`self.RandomExtent`))))))

(event `SetTargetAtMousePosition`
  (bind _returnvalue (`GameplayStatics.GetPlayerController` 0))
  (bind _returnvalue_x (`KismetMathLibrary.BreakVector` (`self.K2_GetActorLocation`)))
  (bind (_locationx _locationy) (`PlayerController.GetMousePosition` _returnvalue))
  (bind (_worldposition _worlddirection) (`GameplayStatics.DeprojectScreenToWorld` _returnvalue (`KismetMathLibrary.MakeVector2D` _locationx _locationy)))
  ;[1 1 1] Set target from mouse / plane intersection
  ;[1 1 1] World location to relative target in blueprint
  (set `self.RelativeTargetY` (.y (`KismetMathLibrary.InverseTransformLocation` (`self.GetTransform`) (`.Intersection` (`KismetMathLibrary.LinePlaneIntersection` _worldposition (+ _worldposition (* _worlddirection 10000.0)) (make `Plane` _returnvalue_x 1.0)))))))

(fn `UserConstructionScript`)