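; Demo actor that compares vector interpolation methods by moving meshes side by side toward a shared target along its local Y axis.
; Each tick runs a custom critically damped spring, VectorSpringInterp with capped delta time, VInterpTo and an uninterpolated reference, plus a debug line.
; Offsets cached at BeginPlay keep the meshes apart.
; A looping timer randomises the target when enabled, and an event can set it from a mouse-ray/plane intersection.
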(event `self.ReceiveBeginPlay`
  ;[1 1 1] Init
  (`self.InitRandomPosition`)
  ;[1 1 1] Register initial offsets
  (for _array_element (`self.K2_GetComponentsByClass` "/Script/Engine.StaticMeshComponent")
    (`BlueprintMapLibrary.Map_Add` (`self.RelativeOffsetMap`) _array_element (`SceneComponent.RelativeLocation` _array_element))))

(event `self.ReceiveTick`
  (params (DeltaSeconds :type "Float (single-precision)"))
  (bind _nointerpolation (`self.NoInterpolation`))
  (bind _vinterpto (`self.VInterpTo`))
  (bind _vectorspringinterp (`self.VectorSpringInterp`))
  (bind _vectorspringinterpcd (`self.VectorSpringInterpCD`))
  (bind _returnvalue (`KismetMathLibrary.TransformLocation` (`self.GetTransform`) (`self.RelativeTarget`)))
  (`|ExecutionSequence`
    (:`then_0`
      ;[0 0.01771 0.004418] VectorSpringInterpCD: Critically Damped Spring (Custom from InterploationLibrary.cpp)
      (`SceneComponent.K2_SetRelativeLocation` _vectorspringinterpcd (`InterpolationLibrary.VectorSpringInterpCD` (`SceneComponent.RelativeLocation` _vectorspringinterpcd) (`self.GetTargetWithOffset` _vectorspringinterpcd) (`self.SpringVelocityCD`) DeltaSeconds) false false))
    (:`then_2`
      ;[1 1 1] VectorSpringInterp (With Critical damping factor at 1!)
      (bind _returnvalue_2 (`KismetMathLibrary.VectorSpringInterp` (`SceneComponent.RelativeLocation` _vectorspringinterp) (`self.GetTargetWithOffset` _vectorspringinterp) (`self.SpringInterpState`) 10.0 1.0 (`KismetMathLibrary.FMin` DeltaSeconds 0.1)))
      (`SceneComponent.K2_SetRelativeLocation` _vectorspringinterp _returnvalue_2 false false))
    (:`then_3`
      ;[1 1 1] VInterpTo
      (`SceneComponent.K2_SetRelativeLocation` _vinterpto (`KismetMathLibrary.VInterpTo` (`SceneComponent.RelativeLocation` _vinterpto) (`self.GetTargetWithOffset` _vinterpto) DeltaSeconds 5.0) false false))
    (:`then_4`
      ;[1 1 1] No Interpolation
      (`SceneComponent.K2_SetRelativeLocation` _nointerpolation (`self.GetTargetWithOffset` _nointerpolation) false false))
    (:`then_5`
      ;[1 1 1] Debug Line
      (`KismetSystemLibrary.DrawDebugLine` (+ _returnvalue (0.0 0.0 -1000.0)) (+ _returnvalue (0.0 0.0 1000.0)) (struct :`R` 1.0 :`G` 1.0 :`B` 1.0 :`A` 1.0) 0.0 5.0))))

(event `InitRandomPosition`
  ;[1 1 1] Random position each X seconds
  (`KismetSystemLibrary.Delay` 1.0)
  (`KismetSystemLibrary.K2_SetTimerDelegate` (delegate `RandomTarget`) 0.7 true))

(event `RandomTarget`
  ;[1 1 1] Random position each X seconds
  (if (`self.RandomEnabled`)
    (set `self.RelativeTarget` (`KismetMathLibrary.MakeVector` 0.0 (* (`KismetMathLibrary.RandomFloat`) (.y (`self.RandomExtent`)))))))

(event `SetTargetAtMousePosition`
  (bind _returnvalue (`GameplayStatics.GetPlayerController` 0))
  (bind _returnvalue_x (`KismetMathLibrary.BreakVector` (`self.K2_GetActorLocation`)))
  (bind (_locationx _locationy) (`PlayerController.GetMousePosition` _returnvalue))
  (bind (_worldposition _worlddirection) (`GameplayStatics.DeprojectScreenToWorld` _returnvalue (`KismetMathLibrary.MakeVector2D` _locationx _locationy)))
  ;[1 1 1] Set target from mouse / plane intersection
  (set `self.RelativeTarget` (`KismetMathLibrary.MakeVector` 0.0 (.y (`KismetMathLibrary.InverseTransformLocation` (`self.GetTransform`) (`.Intersection` (`KismetMathLibrary.LinePlaneIntersection` _worldposition (+ _worldposition (* _worlddirection 10000.0)) (make `Plane` _returnvalue_x 1.0))))))))

(fn `GetTargetWithOffset`
  (params (Mesh :type "StaticMeshComponent Object Reference"))
  (returns (RelativeTarget :type "Vector Structure"))
  (bind (_value _returnvalue) (`BlueprintMapLibrary.Map_Find` (`self.RelativeOffsetMap`) Mesh))
  (if _returnvalue
    (return (+ (`self.RelativeTarget`) _value))
    (else
      (return (`self.RelativeTarget`)))))

(fn `UserConstructionScript`)