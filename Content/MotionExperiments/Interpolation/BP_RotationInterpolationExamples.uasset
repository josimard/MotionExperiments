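; Demo actor that compares rotation interpolation methods side by side on arrow components chasing a shared TargetRotation.
; Tick drives the arrows with a custom critically damped spring, RInterpTo, custom RotatorSlerpTo and an uninterpolated snap.
; A looping timer randomizes the target when RandomEnabled is set.
; SetTargetAtMousePosition instead aims it at the mouse ray's intersection with a vertical plane, avoiding a physics raycast, and draws debug shapes.
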(event `self.ReceiveBeginPlay`
  ;[1 1 1] Init
  (`self.InitRandomPosition`)
  ;[1 1 1] Hide arrows shadows
  (for _array_element (`self.K2_GetComponentsByClass` "/Script/Engine.ArrowComponent")
    (`PrimitiveComponent.SetCastShadow` _array_element false)))

(event `self.ReceiveTick`
  (params (DeltaSeconds :type "Float (single-precision)"))
  (bind _arrow111 (`self.Arrow111`))
  (bind _arrow11 (`self.Arrow11`))
  (bind _arrow1 (`self.Arrow1`))
  (`|ExecutionSequence`
    (:`then_0`
      ;[0 0.01771 0.004418] Critically Damped Spring (Custom 'RotationSpringInterpCD') from InterploationLibrary.cpp
      (bind _returnvalue (`InterpolationLibrary.RotatorSpringInterpCD` (`SceneComponent.RelativeRotation` _arrow111) (`self.TargetRotation`) (`self.SpringVelocity`) DeltaSeconds))
      (`SceneComponent.K2_SetRelativeRotation` _arrow111 _returnvalue false false))
    (:`then_1`
      ;[1 1 1] RInterpTo
      (`SceneComponent.K2_SetRelativeRotation` _arrow1 (`KismetMathLibrary.RInterpTo` (`SceneComponent.RelativeRotation` _arrow1) (`self.TargetRotation`) DeltaSeconds 5.0) false false :!label _label))
    (:`then_2`
      ;[1 1 1] RQuatInterpTo  (Custom from InterploationLibrary.cpp
      (bind _returnvalue_2 (`InterpolationLibrary.RotatorSlerpTo` (`SceneComponent.RelativeRotation` _arrow11) (`self.TargetRotation`) DeltaSeconds))
      (`SceneComponent.K2_SetRelativeRotation` _arrow11 _returnvalue_2 false false))
    (:`then_3`
      (goto _label))
    (:`then_4`
      ;[1 1 1] No Interpolation
      (`SceneComponent.K2_SetRelativeRotation` (`self.Arrow`) (`self.TargetRotation`) false false))))

(event `InitRandomPosition`
  ;[1 1 1] Random rotation
  (`KismetSystemLibrary.Delay` 1.0)
  (`KismetSystemLibrary.K2_SetTimerDelegate` (delegate `RandomTarget`) 1.5 true))

(event `RandomTarget`
  ;[1 1 1] Random rotation
  (if (`self.RandomEnabled`)
    (set `self.TargetRotation` (`KismetMathLibrary.RandomRotator` true))))

(event `SetTargetAtMousePosition`
  (bind _returnvalue (`GameplayStatics.GetPlayerController` 0))
  (bind _returnvalue_x (`KismetMathLibrary.BreakVector` (`self.K2_GetActorLocation`)))
  (bind _defaultsceneroot (`self.DefaultSceneRoot`))
  (bind (_locationx _locationy) (`PlayerController.GetMousePosition` _returnvalue))
  (bind _returnvalue_2 (`SceneComponent.K2_GetComponentLocation` _defaultsceneroot))
  (bind (_worldposition _worlddirection) (`GameplayStatics.DeprojectScreenToWorld` _returnvalue (`KismetMathLibrary.MakeVector2D` _locationx _locationy)))
  (bind _returnvalue_3 (+ (`.Intersection` (`KismetMathLibrary.LinePlaneIntersection` _worldposition (+ _worldposition (* _worlddirection 10000.0)) (make `Plane` _returnvalue_x 1.0))) (-150.0 0.0 0.0)))
  ;[1 1 1] Set target from mouse / plane intersection
  ;[1 1 1] World location to relative target in blueprint
  (set `self.TargetRotation` (`KismetMathLibrary.InverseTransformRotation` (`SceneComponent.K2_GetComponentToWorld` _defaultsceneroot) (`KismetMathLibrary.FindLookAtRotation` _returnvalue_2 _returnvalue_3)))
  (`KismetSystemLibrary.DrawDebugPoint` _returnvalue_3 10.0 (struct :`R` 1.0 :`B` 0.335471 :`A` 1.0))
  (`KismetSystemLibrary.DrawDebugSphere` _returnvalue_2 60.0 3 (struct :`R` 0.291667 :`B` 0.133423 :`A` 1.0) 0.0 5.0))

(fn `UserConstructionScript`)